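; Enemy pawn that hunts the player's ship, orbiting and shooting it once within circling range.
; Each tick it regenerates health, then either steps toward the player with sphere-trace avoidance or circles and fires its child-actor turret on a random cooldown.
; Orbiting attaches the pawn to a rotation point spawned at the player, reversing on obstacles or random timers.
; HealthSubtract applies fixed damage and destroys it at zero; health query functions are stubs.
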(event `MoveToLocation`
  (params (TargetLocation :type "Vector Structure") (StartLocation :type "Vector Structure"))
  (set `self.DirectionToPlayer` (- TargetLocation StartLocation))
  (set `self.MoveLocation` (+ StartLocation (* (`KismetMathLibrary.Normal` (`self.DirectionToPlayer`)) (`self.MovementSpeed`) (`GameplayStatics.GetWorldDeltaSeconds`))))
  (bind _outhit (`KismetSystemLibrary.SphereTraceSingle` :`Start` StartLocation :`End` (`self.MoveLocation`) :`Radius` 100.0 :`TraceChannel` "TraceTypeQuery1" :`DrawDebugType` "ForOneFrame" :`DrawTime` 0.5))
  (bind (_bblockinghit _binitialoverlap _time _distance _location _impactpoint _normal _impactnormal _physmat _hitactor) (`GameplayStatics.BreakHitResult` _outhit))
  (if (!= _hitactor null)
    (bind _output_get (set `self.AdjustedMoveLocation` (+ (`self.MoveLocation`) (* _normal (`self.OffsetDistance`)))))
    (bind (_returnvalue_x _returnvalue_y _returnvalue_z) (`KismetMathLibrary.BreakVector` (`KismetMathLibrary.VInterpTo` StartLocation _output_get)))
    (set `MovementComponent.Velocity` (`KismetMathLibrary.MakeVector` 0.0 _returnvalue_y _returnvalue_z) (`self.FloatingPawnMovement`))
    (else
      (`self.K2_SetActorLocation` (`self.MoveLocation`)))))

(event `MoveToPlayer`
  (set `self.DirectionToPlayer` (- (`self.K2_GetActorLocation` (`self.PlayerRef`)) (`SceneComponent.K2_GetComponentLocation` (`self.Capsule`))))
  (set `self.MoveLocation` (+ (`SceneComponent.K2_GetComponentLocation` (`self.Capsule`)) (* (`KismetMathLibrary.Normal` (`self.DirectionToPlayer`)) (`self.MovementSpeed`) (`GameplayStatics.GetWorldDeltaSeconds`))))
  ;[1 1 1] Avoidng obstacles (need improvements)
  (bind _outhit (`KismetSystemLibrary.SphereTraceSingle` :`Start` (`SceneComponent.K2_GetComponentLocation` (`self.Capsule`)) :`End` (`self.MoveLocation`) :`Radius` 100.0 :`TraceChannel` "TraceTypeQuery1" :`DrawTime` 0.5))
  (bind (_bblockinghit _binitialoverlap _time _distance _location _impactpoint _normal _impactnormal _physmat _hitactor) (`GameplayStatics.BreakHitResult` _outhit))
  (if (!= _hitactor null)
    (bind _output_get (set `self.AdjustedMoveLocation` (+ (`self.MoveLocation`) (* _normal (`self.OffsetDistance`)))))
    (bind (_returnvalue_x _returnvalue_y _returnvalue_z) (`KismetMathLibrary.BreakVector` (`KismetMathLibrary.VInterpTo` (`SceneComponent.K2_GetComponentLocation` (`self.Capsule`)) _output_get)))
    (set `MovementComponent.Velocity` (`KismetMathLibrary.MakeVector` 0.0 _returnvalue_y _returnvalue_z) (`self.FloatingPawnMovement`))
    (else
      (`self.K2_SetActorLocation` (`self.MoveLocation`)))))

(event `OutOfRange`
  (bind _rotpoint (`self.RotPoint`)
    (:`then`
      (`self.K2_DetachFromActor` _rotpoint "KeepWorld" "KeepWorld" "KeepWorld")
      (set `self.IsCircling` false)
      (`/Game/Blueprints/BP_RotPoint.DestroyActor` (`self.RotPoint`)))
    (:`else`)))

(event `self.ReceiveBeginPlay`
  (bind _asbp_turret (cast `/Game/Blueprints/Guns/BP_Turret` (`ChildActorComponent.ChildActor` (`self.Gun`))))
  (set `self.GunRef` _asbp_turret)
  (`self.SetOwner` (`self.GunRef`) self)
  (bind _returnvalue (`GameplayStatics.GetActorOfClass` "/Game/Blueprints/BP_ShipPawn.BP_ShipPawn_C"))
  (set `self.PlayerRef` _returnvalue))

(event `UpdateAI`
  (if (`KismetSystemLibrary.IsValid` (`self.PlayerRef`))
    (set `self.DistanceToPlayer` (`KismetMathLibrary.VSize` (- (`self.K2_GetActorLocation`) (`self.K2_GetActorLocation` (`self.PlayerRef`)))))
    (if (> (`self.DistanceToPlayer`) (`self.CirlingRange`))
      (`self.OutOfRange`)
      (`self.MoveToLocation` (`self.K2_GetActorLocation` (`self.PlayerRef`)) (`SceneComponent.K2_GetComponentLocation` (`self.Capsule`)))
      (else
        (`self.CircleAroundPlayer`)
        (`self.Fire`)))))

(event `self.ReceiveTick`
  (params (DeltaSeconds :type "Float (single-precision)"))
  (`HealthComponent.PassiveHealthRegen` (`self.HealthComponent`) 3.0)
  ;[1 1 1] Movement
  (`self.UpdateAI`))

(event `CircleAroundPlayer`
  ;[1 1 1] Make it smooth
  (if (not (`self.IsCircling`))
    (bind _returnvalue (`|SpawnActorFromClass` "/Game/Blueprints/BP_RotPoint.BP_RotPoint_C" (`self.GetTransform` (`self.PlayerRef`)) "Undefined" "MultiplyWithRoot" null null))
    (bind _output_get (set `self.RotPoint` _returnvalue))
    (`self.K2_AttachToActor` _output_get "None" "KeepWorld" "KeepWorld" "KeepWorld")
    (set `self.IsCircling` true)
    (else
      (bind _outhit (`KismetSystemLibrary.SphereTraceSingle` :`Start` (`SceneComponent.K2_GetComponentLocation` (`self.Capsule`)) :`End` (`self.MoveLocation`) :`Radius` 100.0 :`TraceChannel` "TraceTypeQuery1" :`DrawDebugType` "ForOneFrame" :`DrawTime` 0.5))
      (if (!= (`.HitActor` (`GameplayStatics.BreakHitResult` _outhit)) null)
        (set `self.CircleDirection` (* (`self.CircleDirection`) -1.0)))
      (`SceneComponent.K2_AddLocalRotation` (`Actor.RootComponent` (`self.RotPoint`)) (`KismetMathLibrary.MakeRotator` (`self.CircleDirection`)) false false)
      (if (not (`self.IsRandPosTimerHandleRunning`))
        (set `self.IsRandPosTimerHandleRunning` true)
        (bind _returnvalue_2 (`KismetSystemLibrary.K2_SetTimerDelegate` (delegate `RandDirection`) (`KismetMathLibrary.RandomFloatInRange` 1.0 3.0)))
        (set `self.RandomPositionTimerHandle` _returnvalue_2)))))

(event `OnCooldownTimer`
  (set `self.GunOnCooldown` false)
  (`KismetSystemLibrary.K2_ClearAndInvalidateTimerHandle` (`self.OnCooldownTimerHandle`)))

(event `RandDirection`
  (if (> (`KismetMathLibrary.RandomFloatInRange` -5.0 5.0) 0.0)
    (set `self.CircleDirection` 1.0)
    (else
      (set `self.CircleDirection` -1.0)))
  (set `self.IsRandPosTimerHandleRunning` false))

(event `Fire`
  (if (not (`self.GunOnCooldown`))
    (set `self.GunOnCooldown` true)
    (`self.FireTheGun`)
    (bind _returnvalue (`KismetSystemLibrary.K2_SetTimerDelegate` (delegate `CustomEvent`) (`KismetMathLibrary.RandomFloatInRange` 3.0 5.0)))
    (set `self.OnCooldownTimerHandle` _returnvalue)))

(event `FireTheGun`
  (`/Game/Blueprints/Guns/BP_Turret.FireTheGun` (`self.GunRef`) self (`self.PlayerRef`)))

(event `CustomEvent`
  (set `self.GunOnCooldown` false)
  (`KismetSystemLibrary.K2_ClearAndInvalidateTimerHandle` (`self.OnCooldownTimerHandle`)))

(event `/Game/Blueprints/DamageSystem/BPI_Health.SubtractHealth`)

(event `self.HealthSubtract`
  (`HealthComponent.TakeDamage` (`self.HealthComponent`) 20.0)
  (`HealthComponent.SetRegenCooldown` (`self.HealthComponent`))
  (if (`HealthComponent.IsHealthZero` (`self.HealthComponent`))
    (`self.K2_DestroyActor`)))

(fn `GetCurrentHealth`
  (returns (CurrentHealth :type "Float (double-precision)"))
  (return 0.0))

(fn `GetMaxHealth`
  (returns (MaxHealth :type "Float (double-precision)"))
  (return 0.0))

(fn `Heal`
  (params (Amount :type "Float (double-precision)" :default 0.0))
  (returns (NewHealth :type "Float (double-precision)"))
  (return 0.0))

(fn `IsDead`
  (returns (IsDead :type Boolean))
  (return false))

(fn `TakeDamage`
  (params (Damage :type "Float (double-precision)" :default 0.0))
  (returns (WasDamaged :type Boolean))
  (return false))

(fn `UserConstructionScript`)