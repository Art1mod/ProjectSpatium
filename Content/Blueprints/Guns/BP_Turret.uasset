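; Turret actor with a barrel that rotates and fires projectiles, exposing functions without driving them from its own event graph.
; FireTheGun spawns a BP_ProjectileBase at ShootPoint with the given owner, then blocks firing for CooldownTime, using a timer and the CanFire flag.
; RotateToTarget eases barrel pitch toward the first player's pawn with RInterpTo, while RotateBarrel adds a local roll.
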(event `self.ReceiveBeginPlay`)

(event `ResetFire`
  (set `self.CanFire` true))

(fn `FireTheGun`
  (params (Owner :type "Actor Object Reference"))
  (if (`self.CanFire`)
    (bind _returnvalue (`|SpawnActorFromClass` "/Game/InfinityBladeEffects/Projectiles/BP_ProjectileBase.BP_ProjectileBase_C" (`SceneComponent.K2_GetComponentToWorld` (`self.ShootPoint`)) "AdjustIfPossibleButAlwaysSpawn" "MultiplyWithRoot" Owner 1000.0 0.0 null false null))
    (`self.SetOwner` _returnvalue Owner)
    (set `self.CanFire` false)
    (`KismetSystemLibrary.K2_SetTimerDelegate` (`|CreateDelegate` :!event `ResetFire`) (`self.CooldownTime`))))

(fn `RotateBarrel`
  (params (Rotation :type "Float (double-precision)"))
  (`SceneComponent.K2_AddLocalRotation` (`self.Barrel`) (`KismetMathLibrary.MakeRotator` Rotation) false false))

(fn `RotateToTarget`
  (bind (_returnvalue_roll _returnvalue_pitch) (`KismetMathLibrary.BreakRotator` (`KismetMathLibrary.RInterpTo` (`SceneComponent.K2_GetComponentRotation` (`self.Barrel`)) (`KismetMathLibrary.FindLookAtRotation` (`self.K2_GetActorLocation`) (`self.K2_GetActorLocation` (`GameplayStatics.GetPlayerPawn` 0))) (`GameplayStatics.GetWorldDeltaSeconds`) 1.0)))
  (`SceneComponent.K2_SetRelativeRotation` (`self.Barrel`) (`KismetMathLibrary.MakeRotator` 0.0 _returnvalue_pitch) false false))

(fn `UserConstructionScript`)